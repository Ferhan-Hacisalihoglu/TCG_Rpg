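; BP_Card is a physical card actor for the TCG game that displays a card and animates it being played.
; On BeginPlay it builds front and back widgets from CardInfo, assigns them to widget components and sets a one-minute lifespan.
; API_PlayCardAnimation rolls the card over, then chains two timelines to move it to the target and flip it back.
; It finally simulates physics briefly so the card can settle.
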(event `self.ReceiveBeginPlay`
  (bind _cardinfo (`self.CardInfo`))
  (bind _main_widget_ref (`self.Main Widget Ref`))
  (bind (_name _description _type _cardcost _icon _cardreuirementleft _cardreuirementright _wbp_backofcard _wbp_frontofcard) (break `/Game/_Main/GameMode/TCGGame/Varaibles/ST_Card` _cardinfo))
  ; Start the card information
  (bind _returnvalue (`|CreateWidget` _wbp_backofcard null _cardinfo _main_widget_ref))
  (`/Game/_Main/GameMode/TCGGame/Widget/CardTypes/WBP_Card.API_LoadCardStyle` _returnvalue)
  (`WidgetComponent.SetWidget` (`self.BackOfTheCard`) _returnvalue)
  (bind _returnvalue_2 (`|CreateWidget` _wbp_frontofcard null _cardinfo _main_widget_ref))
  (`/Game/_Main/GameMode/TCGGame/Widget/CardTypes/WBP_Card.API_LoadCardStyle` _returnvalue_2)
  (`WidgetComponent.SetWidget` (`self.FrontOfTheCard`) _returnvalue_2)
  (`self.SetLifeSpan` 60.0))

(event `API_PlayCardAnimation`
  (params (FinalTransform :type "Transform Structure"))
  (bind _returnvalue (`self.K2_GetActorRotation` self))
  ; When player place card we play the animation and fx here
  (`self.K2_SetActorRotation` self (`KismetMathLibrary.MakeRotator` 180.0 (.pitch (.rotation FinalTransform)) (.yaw (.rotation FinalTransform))) false)
  (bind (_direction _moveto) (`Timeline|MoveCardTo` :!via `PlayFromStart`)
    (:`Update`
      (`self.K2_SetActorLocation` self (`KismetMathLibrary.VLerp` (`self.K2_GetActorLocation` self) (.location FinalTransform) _moveto) false false))
    (:`Finished`
      (bind (_direction_2 _moveto_2) (`Timeline|RotateCard` :!via `PlayFromStart`)
        (:`Update`
          (`self.K2_SetActorRotation` self (`KismetMathLibrary.RLerp` _returnvalue (`KismetMathLibrary.MakeRotator` 0.0 (.pitch _returnvalue) (.yaw _returnvalue)) _moveto_2) false))
        (:`Finished`
          (`PrimitiveComponent.SetSimulatePhysics` (`self.BaseCard`) true)
          (`KismetSystemLibrary.Delay` 0.5)
          (`PrimitiveComponent.SetSimulatePhysics` (`self.BaseCard`) false))))))

(fn `UserConstructionScript`)
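; Player component for a multiplayer trading card game, holding a human or AI player's deck, cards and attributes.
; Relays actions through Client, Server and Multicast events, with GameMode handling turns, dice, damage and syncing.
; Card use checks turn and mana, then applies costs and effects; attribute rules let one stat shield another.
; Also drives the main widget and 3D card spawning, with dev-only random names and decks.
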(event `API_StartAI`
  ; Start the widget for the player
  (`self.API_FirstLoadPlayerAttributes_Client`))

(event `API_StartTCG`
  (params (Controller :type "Controller Object Reference"))
  ; Start the widget for the player
  (set `self.Controller` Controller)
  (bind _returnvalue (`|CreateWidget` "/Game/_Main/GameMode/TCGGame/Widget/WBP_MainTcg.WBP_MainTcg_C" null self))
  (bind _output_get (set `self.WidgetRef` _returnvalue))
  (`UserWidget.AddToViewport` _output_get 0)
  (`self.API_FirstLoadPlayerAttributes_Client`)
  ; This is only for dev
  (for _ (range 1 (+ (`.MaxCards_12_8D1A36F54D25B81E172CA39736C3500C` (break `/Game/_Main/GameMode/TCGGame/Varaibles/ST_TCGSettings` (`self.TCG_Settings`))) 1))
    (bind _outrownames (`DataTableFunctionLibrary.GetDataTableRowNames` "/Game/_Main/GameMode/TCGGame/Varaibles/DT_Card.DT_Card"))
    (`KismetArrayLibrary.Array_Add` (`.cardDeck_23_8991139749678E699F778EB1FA09F988` (break `/Game/_Main/GameMode/TCGGame/Varaibles/ST_PlayerInfo` (`self.PlayerInfo`))) (make `DataTableRowHandle` "/Game/_Main/GameMode/TCGGame/Varaibles/DT_Card.DT_Card" (`KismetArrayLibrary.Array_Random` _outrownames)))))

(event `API_FirstLoadPlayerAttributes_Client`
  ; Load player attributes
  (`self.API_FirstLoadPlayerAttributes_Server`))

(event `API_FirstLoadPlayerAttributes_Server`
  ; Load player attributes
  (`self.API_FirstLoadPlayerAttributes_Multicast`)
  (bind _asgs_tcggame_state (cast `/Game/_Main/GameMode/TCGGame/GameMode/GS_TCGGame_State` (`GameplayStatics.GetGameState`)))
  (set `self.GameState` _asgs_tcggame_state)
  (bind _asgm_tcg_game (cast `/Game/_Main/GameMode/TCGGame/GameMode/GM_TcgGame` (`GameplayStatics.GetGameMode`)))
  (set `self.GameMode` _asgm_tcg_game))

(event `API_FirstLoadPlayerAttributes_Multicast`
  ; Load player attributes
  (setmembers `/Game/_Main/GameMode/TCGGame/Varaibles/ST_PlayerInfo` :`StructRef` (`self.PlayerInfo`) :`playerName` (select `int` (`KismetMathLibrary.RandomInteger` 3) :`0` "test 01" :`1` "test 02" :`2` "test 03" :`3` "test 04") :`playerID` (`KismetSystemLibrary.MakeLiteralString` (`KismetStringLibrary.Concat_StrStr` (`KismetStringLibrary.Conv_IntToString` (`KismetMathLibrary.RandomIntegerInRange` 1 999)) (`KismetStringLibrary.Conv_IntToString` (`KismetMathLibrary.RandomIntegerInRange` 1 999)))))
  (for _array_element (`.defaultAttributes_13_BDFE291241C6477CE407E98FAB363C96` (break `/Game/_Main/GameMode/TCGGame/Varaibles/ST_PlayerInfo` (`self.PlayerInfo`)))
    (bind _returnvalue (`|GetDataTableRow` "/Game/_Main/GameMode/TCGGame/Varaibles/DT_PlayerAttributes.DT_PlayerAttributes" (`.RowName` (break `DataTableRowHandle` _array_element)))
      (:`then`
        (`KismetArrayLibrary.Array_AddUnique` (`.playerAttribute_12_1398B0B949EE9B8A2B8F089301723C01` (break `/Game/_Main/GameMode/TCGGame/Varaibles/ST_PlayerInfo` (`self.PlayerInfo`))) _returnvalue))))
  (`self.API_SyncClients_Client`))

(event `API_MoveCardToPositionAnimated`
  (params (Target :type "CanvasPanelSlot Object Reference") (PositionX :type "Float (double-precision)") (PositionY :type "Float (double-precision)"))
  ; Card FX move the card to the position
  (bind _returnvalue (`|SpawnActorFromClass` "/Game/_Main/GameMode/TCGGame/Actor/BP_CardInstance.BP_CardInstance_C" (`KismetMathLibrary.MakeTransform` (0.0 0.0 0.0)) "Undefined" "MultiplyWithRoot" null null))
  (`/Game/_Main/GameMode/TCGGame/Actor/BP_CardInstance.API_MoveCardToPositionAnimated` _returnvalue Target PositionX PositionY))

(event `API_SetTimeLeftWidget_Client`
  (bind _widgetref (`self.WidgetRef`))
  ; Display how much time left we have
  (`/Engine/EditorBlueprintResources/StandardMacros.IsValid` _widgetref
    (:`Is Valid`
      (`/Game/_Main/GameMode/TCGGame/Widget/WBP_MainTcg.API_SetTurnLeft` _widgetref))))

(event `API_ReloadWidget_Client`
  ; Reload the tcg widget informayion
  (`self.API_ReloadWidget_Server`))

(event `API_SetAndRefreshEnemy_Server`
  (params (Enemy :type "/Game/_Main/GameMode/TCGGame/GameMode/BPC_TCG_Component Object Reference"))
  ; Reload the tcg widget informayion
  ;; Call back from game mode set enemy info
  (`/Engine/EditorBlueprintResources/StandardMacros.IsValid` Enemy
    (:`Is Valid`
      (`self.API_SetAndRefreshEnemy_Multicast` (`/Game/_Main/GameMode/TCGGame/GameMode/BPC_TCG_Component.PlayerInfo` Enemy)))))

(event `API_ReloadWidget_Server`
  (bind _gamemode (`self.GameMode`))
  ; Reload the tcg widget informayion
  (`/Engine/EditorBlueprintResources/StandardMacros.IsValid` _gamemode
    (:`Is Valid`
      (`/Game/_Main/GameMode/TCGGame/GameMode/GM_TcgGame.API_FindEnemy` _gamemode self))))

(event `API_SetAndRefreshEnemy_Multicast`
  (params (EnemyInfo :type "/Game/_Main/GameMode/TCGGame/Varaibles/ST_PlayerInfo Structure"))
  ; Reload the tcg widget informayion
  ;; Call back from game mode set enemy info
  (set `self.EnemyInfo` EnemyInfo)
  (`self.API_ReloadWidget_Multicast`))

(event `API_ReloadWidget_Multicast`
  (bind _widgetref (`self.WidgetRef`))
  ; Reload the tcg widget informayion
  (`/Engine/EditorBlueprintResources/StandardMacros.IsValid` _widgetref
    (:`Is Valid`
      (`/Game/_Main/GameMode/TCGGame/Widget/WBP_MainTcg.API_ReloadWidget` _widgetref (`self.EnemyInfo`)))))

(event `API_SyncClients_Client`
  ; Reload the tcg widget informayion
  ;; Sync all client data
  (`self.API_SyncClients_Server`))

(event `API_SyncClients_Server`
  (bind _gamemode (`self.GameMode`))
  ; Reload the tcg widget informayion
  ;; Sync all client data
  (`/Engine/EditorBlueprintResources/StandardMacros.IsValid` _gamemode
    (:`Is Valid`
      (`/Game/_Main/GameMode/TCGGame/GameMode/GM_TcgGame.API_SyncClients` _gamemode))))

(event `API_RollDice`
  ; Roll dice on the server
  (`self.API_RollDice_Server`))

(event `API_RollDice_Server`
  (bind _gamemode (`self.GameMode`))
  ; Roll dice on the server
  (`/Game/_Main/GameMode/TCGGame/GameMode/GM_TcgGame.API_Roll_Dice` _gamemode)
  (`self.API_RollDice_Multicast` (`/Game/_Main/GameMode/TCGGame/GameMode/GM_TcgGame.LastDiceRoll` _gamemode)))

(event `API_RollDice_Multicast`
  (params (DiceRoll :type Integer))
  (bind _wbp_dice (`/Game/_Main/GameMode/TCGGame/Widget/WBP_MainTcg.WBP_Dice` (`self.WidgetRef`)))
  ; Roll dice on the server
  (`/Engine/EditorBlueprintResources/StandardMacros.IsValid` _wbp_dice
    (:`Is Valid`
      (set `/Game/_Main/GameMode/TCGGame/Widget/WBP_Dice.DiceRoll` DiceRoll _wbp_dice))))

(event `API_AddDrawNewCard_Client`
  ;[0.15 0.0375 0.15 0.5] When the player or the system add a new card
  (`self.API_AddDrawNewCard_Server`))

(event `API_AddNewCardAction_Client`
  (params (Card :type "/Game/_Main/GameMode/TCGGame/Varaibles/ST_Card Structure") (DeckIndex :type Integer))
  ;[0.15 0.0375 0.15 0.5] When the player or the system add a new card
  ;; Sync added player card on all clients and server
  (`self.API_AddNewCardAction_Server` Card DeckIndex))

(event `API_AddDrawNewCard_Server`
  ;[0.15 0.0375 0.15 0.5] When the player or the system add a new card
  (`self.API_AddDrawNewCard_Multicast`))

(event `API_AddNewCardAction_Server`
  (params (Card :type "/Game/_Main/GameMode/TCGGame/Varaibles/ST_Card Structure") (DeckIndex :type Integer))
  ;[0.15 0.0375 0.15 0.5] When the player or the system add a new card
  ;; Sync added player card on all clients and server
  (`self.API_AddNewCardAction_Multicast` Card DeckIndex))

(event `API_AddNewCardAction_Multicast`
  (params (Card :type "/Game/_Main/GameMode/TCGGame/Varaibles/ST_Card Structure") (DeckIndex :type Integer))
  (bind _widgetref (`self.WidgetRef`))
  (bind ((`cards_18_47C47CEB40F75F324BDE94B4887DC6EC` _cards) (`cardRecived_26_952C37404E9F230D4901C78C5ABB8D0A` _cardrecived)) (break `/Game/_Main/GameMode/TCGGame/Varaibles/ST_PlayerInfo` (`self.PlayerInfo`)))
  ;[0.15 0.0375 0.15 0.5] When the player or the system add a new card
  ;; Sync added player card on all clients and server
  (`KismetArrayLibrary.Array_Add` _cards Card)
  (`/Engine/EditorBlueprintResources/StandardMacros.IncrementInt` _cardrecived
    (:`  `
      (`/Engine/EditorBlueprintResources/StandardMacros.IsValid` _widgetref
        (:`Is Valid`
          (`/Game/_Main/GameMode/TCGGame/Widget/WBP_MainTcg.API_AddNewCard` _widgetref Card))
        (:`Is Not Valid`
          _))
      (`KismetArrayLibrary.Array_Remove` _cards DeckIndex)
      (`self.API_SyncClients_Client`))))

(event `API_AddDrawNewCard_Multicast`
  (bind (_outitem _outindex) (`KismetArrayLibrary.Array_Random` (`.cardDeck_23_8991139749678E699F778EB1FA09F988` (break `/Game/_Main/GameMode/TCGGame/Varaibles/ST_PlayerInfo` (`self.PlayerInfo`)))))
  ;[0.15 0.0375 0.15 0.5] When the player or the system add a new card
  (bind _returnvalue (`|GetDataTableRow` "/Game/_Main/GameMode/TCGGame/Varaibles/DT_Card.DT_Card" (`.RowName` (break `DataTableRowHandle` _outitem)))
    (:`then`
      (`self.API_AddNewCardAction_Client` _returnvalue _outindex))))

(event `API_EndTurn_Client`
  ; When player ends turn
  (`self.API_EndTurn_Server`))

(event `API_EndTurn_Server`
  ; When player ends turn
  (`self.MC_HasTurnPermission`
    (:`True`
      (`/Game/_Main/GameMode/TCGGame/GameMode/GM_TcgGame.API_EndPlayerTurn` (`self.GameMode`)))))

(event `API_AddAtribute_Client`
  (params (Attribute :type "/Game/_Main/GameMode/TCGGame/Varaibles/E_PlayerAttribute Enum" :default "NewEnumerator0") (Amount :type Integer))
  ;[0.0375 0.15 0.0375 0.502] When we add attribute
  (`self.API_AddAtribute_Server` Attribute Amount))

(event `API_UseCard`
  (params (`Card Widget` :type "/Game/_Main/GameMode/TCGGame/Widget/CardTypes/WBP_Card Object Reference"))
  ;[0.15 0.15 0.0375 0.5] Remove the card from  the player deck
  (bind _output_get (set `self.LastPlayCard` `Card Widget`))
  (`self.API_UseCard_Server` (`/Game/_Main/GameMode/TCGGame/Widget/CardTypes/WBP_Card.CardData` _output_get)))

(event `API_Spawn3DCard_Client`
  (params (CardInfo :type "/Game/_Main/GameMode/TCGGame/Varaibles/ST_Card Structure") (isEnemy :type Boolean))
  ;[0.15 0.15 0.0375 0.5] Remove the card from  the player deck
  ;; Spawn 3d asset
  (`self.API_Spawn3DCard_Server` CardInfo isEnemy))

(event `API_AddAtribute_Server`
  (params (Attribute :type "/Game/_Main/GameMode/TCGGame/Varaibles/E_PlayerAttribute Enum" :default "NewEnumerator0") (Amount :type Integer))
  ;[0.0375 0.15 0.0375 0.502] When we add attribute
  (`self.API_AddAtribute_Multicast` Attribute Amount))

(event `API_StartCardCustomRule_Client`
  (params (CardInfo :type "/Game/_Main/GameMode/TCGGame/Varaibles/ST_Card Structure"))
  ;[0.15 0.15 0.0375 0.5] Remove the card from  the player deck
  (`self.API_StartCardCustomRule_Server` CardInfo))

(event `API_AddAtribute_Multicast`
  (params (Attribute :type "/Game/_Main/GameMode/TCGGame/Varaibles/E_PlayerAttribute Enum" :default "NewEnumerator0") (Amount :type Integer))
  ;[0.0375 0.15 0.0375 0.502] When we add attribute
  (for (_array_element _array_index) (`.playerAttribute_12_1398B0B949EE9B8A2B8F089301723C01` (break `/Game/_Main/GameMode/TCGGame/Varaibles/ST_PlayerInfo` (`self.PlayerInfo`)))
    (if (`|EnumEquality` (`.name_12_77F2DFD944D268F5A3B1679009ADE39A` (break `/Game/_Main/GameMode/TCGGame/Varaibles/ST_PlayerAttributes` _array_element)) Attribute)
      (bind ((`max_8_35DF50BA405651E22E5F40B94618A4CF` _max) (`current_11_F36D572A4C9F9C60EB314AB5DA8DC1DE` _current)) (break `/Game/_Main/GameMode/TCGGame/Varaibles/ST_PlayerAttributes` _array_element))
      (bind _returnvalue (+ _current Amount))
      (setmembers `/Game/_Main/GameMode/TCGGame/Varaibles/ST_PlayerAttributes` :`StructRef` (`|GetArrayItem` (`.playerAttribute_12_1398B0B949EE9B8A2B8F089301723C01` (break `/Game/_Main/GameMode/TCGGame/Varaibles/ST_PlayerInfo` (`self.PlayerInfo`))) _array_index) :`current` (`KismetMathLibrary.SelectInt` _max _returnvalue (>= _returnvalue _max)))
      (break)))
  (`self.API_SyncClients_Client`))

(event `API_Spawn3DCard_Server`
  (params (CardInfo :type "/Game/_Main/GameMode/TCGGame/Varaibles/ST_Card Structure") (isEnemy :type Boolean))
  ;[0.15 0.15 0.0375 0.5] Remove the card from  the player deck
  ;; Spawn 3d asset
  (`self.API_Spawn3DCard_Multicast` CardInfo isEnemy))

(event `API_StartCardCustomRule_Server`
  (params (CardInfo :type "/Game/_Main/GameMode/TCGGame/Varaibles/ST_Card Structure"))
  ;[0.15 0.15 0.0375 0.5] Remove the card from  the player deck
)

(event `API_Spawn3DCard_Multicast`
  (params (CardInfo :type "/Game/_Main/GameMode/TCGGame/Varaibles/ST_Card Structure") (isEnemy :type Boolean))
  ;[0.15 0.15 0.0375 0.5] Remove the card from  the player deck
  ;; Spawn 3d asset
  (`self.FN_Spawn3DCardOnArea` CardInfo isEnemy))

(event `API_UseCard_Server`
  (params (CardData :type "/Game/_Main/GameMode/TCGGame/Varaibles/ST_Card Structure"))
  ;[0.15 0.15 0.0375 0.5] Remove the card from  the player deck
  (`self.MC_HasTurnPermission`
    (:`True`
      (if (>= (`.current_11_F36D572A4C9F9C60EB314AB5DA8DC1DE` (break `/Game/_Main/GameMode/TCGGame/Varaibles/ST_PlayerAttributes` (`self.FN_GetPlayerAttribute` "NewEnumerator1"))) (`.cardCost_19_E3744B754EDC90550D965EA37D03EAE0` (break `/Game/_Main/GameMode/TCGGame/Varaibles/ST_Card` CardData)))
        (`self.API_UseCard_Multicast` CardData)
        (else
          (`self.API_SendNotification` "NewEnumerator1" "You don't have enough mana."))))))

(event `API_SendNotification`
  (params (Type :type "/Game/_Main/GameMode/TCGGame/Varaibles/E_NotificationType Enum" :default "NewEnumerator0") (Description :type Text))
  ;[0.15 0.15 0.0375 0.5] Remove the card from  the player deck
  (`/Game/_Main/GameMode/TCGGame/Widget/WBP_MainTcg.API_DisplayNotification` (`self.WidgetRef`) Type Description))

(event `API_RemoveAttribute_Client`
  (params (Attribute :type "/Game/_Main/GameMode/TCGGame/Varaibles/E_PlayerAttribute Enum" :default "NewEnumerator0") (Amount :type Integer) (SkipRule :type Boolean :default true))
  ;[0.15 0.0375 0.0375 0.502] Decrese attribute
  (`self.API_RemoveAttribute_Server` Attribute Amount SkipRule))

(event `API_RemoveAttribute_Server`
  (params (Attribute :type "/Game/_Main/GameMode/TCGGame/Varaibles/E_PlayerAttribute Enum" :default "NewEnumerator0") (Amount :type Integer) (SkipRule :type Boolean :default true))
  ;[0.15 0.0375 0.0375 0.502] Decrese attribute
  (`self.API_RemoveAttribute_Multicast` Attribute Amount SkipRule))

(event `API_UseCard_Multicast`
  (params (CardInfo :type "/Game/_Main/GameMode/TCGGame/Varaibles/ST_Card Structure"))
  (bind _lastplaycard (`self.LastPlayCard`))
  (bind _gamemode (`self.GameMode`))
  ;[0.15 0.15 0.0375 0.5] Remove the card from  the player deck
  ;; Remove the card cost first
  (`self.FN_UseCardAttribute` (make `/Game/_Main/GameMode/TCGGame/Varaibles/ST_CardRequired` false "NewEnumerator1" (`.cardCost_19_E3744B754EDC90550D965EA37D03EAE0` (break `/Game/_Main/GameMode/TCGGame/Varaibles/ST_Card` CardInfo))))
  (for (_array_element _array_index) (`.cards_18_47C47CEB40F75F324BDE94B4887DC6EC` (break `/Game/_Main/GameMode/TCGGame/Varaibles/ST_PlayerInfo` (`self.PlayerInfo`)))
    (if (== (`.name_6_F5CC21EE44CC78742BE808871494189D` (break `/Game/_Main/GameMode/TCGGame/Varaibles/ST_Card` _array_element)) (`.name_6_F5CC21EE44CC78742BE808871494189D` (break `/Game/_Main/GameMode/TCGGame/Varaibles/ST_Card` CardInfo)))
      (`/Engine/EditorBlueprintResources/StandardMacros.IsValid` _gamemode
        (:`Is Valid`
          (`/Game/_Main/GameMode/TCGGame/GameMode/GM_TcgGame.API_PlayerUserCard` _gamemode _array_element self))
        (:`Is Not Valid`
          _))
      (bind ((`cardReuirementLeft_12_59F95E1C4E62C1644F75F6BA04A5AC06` _cardreuirementleft) (`cardReuirementRight_14_DB3FFAD541E2E3EB2C6F5B8336358C02` _cardreuirementright)) (break `/Game/_Main/GameMode/TCGGame/Varaibles/ST_Card` _array_element))
      (`self.FN_UseCardAttribute` _cardreuirementleft)
      (`self.FN_UseCardAttribute` _cardreuirementright)
      ;; Remove the card from the widget if on client mode
      (`/Engine/EditorBlueprintResources/StandardMacros.IsValid` _lastplaycard
        (:`Is Valid`
          (`/Game/_Main/GameMode/TCGGame/Widget/WBP_MainTcg.FN_RemoveCardFromWidget` (`self.WidgetRef`) _lastplaycard))
        (:`Is Not Valid`
          _))
      (`KismetArrayLibrary.Array_Remove` (`.cards_18_47C47CEB40F75F324BDE94B4887DC6EC` (break `/Game/_Main/GameMode/TCGGame/Varaibles/ST_PlayerInfo` (`self.PlayerInfo`))) _array_index)
      (break)))
  (`self.API_SyncClients_Client`))

(event `API_RemoveAttribute_Multicast`
  (params (Attribute :type "/Game/_Main/GameMode/TCGGame/Varaibles/E_PlayerAttribute Enum" :default "NewEnumerator0") (Amount :type Integer) (SkipRule :type Boolean :default true))
  ;[0.15 0.0375 0.0375 0.502] Decrese attribute
  (`self.FN_RemoveAttribute` Attribute Amount SkipRule))

(event `API_ApplyDamage_Client`
  (params (Damage :type Integer))
  ; Apply Damage to Enemy
  (`self.API_ApplyDamage_Server` Damage))

(event `API_ApplyDamage_Server`
  (params (Damage :type Integer))
  ; Apply Damage to Enemy
  (`/Game/_Main/GameMode/TCGGame/GameMode/GM_TcgGame.API_ApplyDamageEnemy` (`self.GameMode`) self Damage))

(event `API_HandleSession_Client`
  ; Create player session
  (bind _asgi_tcggame_instance (cast `/Game/_Main/GameMode/GI_TCGGameInstance` (`GameplayStatics.GetGameInstance`)))
  (set `self.GameInstance` _asgi_tcggame_instance)
  (bind _asplayer_controller (cast `PlayerController` (`self.Controller`)))
  (`CreateSessionCallbackProxy.CreateSession` _asplayer_controller 1 true
    (:`OnSuccess`
      (`KismetSystemLibrary.PrintString` "Online"))
    (:`OnFailure`
      (`KismetSystemLibrary.PrintString` "Fail"))))

(fn `FN_GetNextSpawnPlace`
  (params (isEnemy :type Boolean))
  (returns (OutActors :type "Actor Object Reference"))
  (bind _outactors (`GameplayStatics.GetAllActorsOfClass` (select `bool` isEnemy :`false` "/Game/_Main/GameMode/TCGGame/Actor/BP_PlayerCardSpawn.BP_PlayerCardSpawn_C" :`true` "/Game/_Main/GameMode/TCGGame/Actor/BP_EnemyCardSpawn.BP_EnemyCardSpawn_C" :!type "Actor Class Reference")))
  (return (`KismetArrayLibrary.Array_Random` _outactors)))

(fn `FN_GetPlayerAttribute`
  (params (AttributeName :type "/Game/_Main/GameMode/TCGGame/Varaibles/E_PlayerAttribute Enum" :default "NewEnumerator0"))
  (returns (PlayerAttribute :type "/Game/_Main/GameMode/TCGGame/Varaibles/ST_PlayerAttributes Structure") (PlayerAttributeIndex :type Integer) (IsAttributeValid :type Boolean))
  (locals (Attribute :type "/Game/_Main/GameMode/TCGGame/Varaibles/ST_PlayerAttributes Structure") (AttributeIndex :type Integer) (IsValid :type Boolean))
  (for (_array_element _array_index) (`.playerAttribute_12_1398B0B949EE9B8A2B8F089301723C01` (break `/Game/_Main/GameMode/TCGGame/Varaibles/ST_PlayerInfo` (`self.PlayerInfo`)))
    (if (`|EnumEquality` (`.name_12_77F2DFD944D268F5A3B1679009ADE39A` (break `/Game/_Main/GameMode/TCGGame/Varaibles/ST_PlayerAttributes` _array_element)) AttributeName)
      (set `local.Attribute` _array_element)
      (set `local.AttributeIndex` _array_index)
      (set `local.IsValid` true)
      (break)))
  (return (`local.Attribute`) (`local.AttributeIndex`) (`local.IsValid`)))

(fn `FN_HandleAttributeRule`
  (params (Rules :type "Array of /Game/_Main/GameMode/TCGGame/Varaibles/ST_AttributeRule Structure") (RemoveAttributeAmount :type Integer) (CurrentAttributeAmount :type Integer) (OriginalAttribute :type "/Game/_Main/GameMode/TCGGame/Varaibles/E_PlayerAttribute Enum" :default "NewEnumerator0"))
  (locals (RemoveAttribute :type Integer) (CurrentAttribute :type Integer) (PlayerOriginalAttribute :type "/Game/_Main/GameMode/TCGGame/Varaibles/E_PlayerAttribute Enum" :default "NewEnumerator0") (CurrentAttributeRule :type "/Game/_Main/GameMode/TCGGame/Varaibles/ST_AttributeRule Structure") (CurrentLoopAttribute :type "/Game/_Main/GameMode/TCGGame/Varaibles/ST_PlayerAttributes Structure"))
  (bind ((`name_12_77F2DFD944D268F5A3B1679009ADE39A` _name) (`current_11_F36D572A4C9F9C60EB314AB5DA8DC1DE` _current)) (break `/Game/_Main/GameMode/TCGGame/Varaibles/ST_PlayerAttributes` (`local.CurrentLoopAttribute`)))
  (bind ((`name_12_77F2DFD944D268F5A3B1679009ADE39A` _name_2) (`current_11_F36D572A4C9F9C60EB314AB5DA8DC1DE` _current_2)) (break `/Game/_Main/GameMode/TCGGame/Varaibles/ST_PlayerAttributes` (`local.CurrentLoopAttribute`)))
  (set `local.RemoveAttribute` RemoveAttributeAmount)
  (set `local.CurrentAttribute` CurrentAttributeAmount)
  (set `local.PlayerOriginalAttribute` OriginalAttribute)
  (for _array_element Rules
    (bind _output_get (set `local.CurrentAttributeRule` _array_element))
    (bind (_attribute _rule) (break `/Game/_Main/GameMode/TCGGame/Varaibles/ST_AttributeRule` _output_get))
    (switch `/Game/_Main/GameMode/TCGGame/Varaibles/E_RuleActionAttribute` _rule
      (:`NewEnumerator0`
        (bind _output_get_2 (set `local.CurrentLoopAttribute` (`self.FN_GetPlayerAttribute` _attribute)))
        ; We only want to run this once
        (`/Engine/EditorBlueprintResources/ActorComponentMacros.Switch Has Authority`
          (:`Authority`
            (bind _returnvalue (- (`.current_11_F36D572A4C9F9C60EB314AB5DA8DC1DE` (break `/Game/_Main/GameMode/TCGGame/Varaibles/ST_PlayerAttributes` _output_get_2)) (`local.RemoveAttribute`)))
            (if (== _returnvalue 0)
              ; If is zero it means we have all other attribute amount as sheild
              (`self.API_RemoveAttribute_Client` _name_2 _current_2)
              (elif (<= _returnvalue 0)
                ; Remove all amount of attribute remaning and use negative value to remove sheild attribute
                (`self.API_RemoveAttribute_Client` _name _current)
                (`self.API_RemoveAttribute_Client` (`local.PlayerOriginalAttribute`) (`KismetMathLibrary.Abs_Int` _returnvalue))
                (else
                  ; We just remove amount
                  (`self.API_RemoveAttribute_Client` (`.name_12_77F2DFD944D268F5A3B1679009ADE39A` (break `/Game/_Main/GameMode/TCGGame/Varaibles/ST_PlayerAttributes` (`local.CurrentLoopAttribute`))) (`local.RemoveAttribute`)))))))))))

(fn `FN_IsMyTurn`
  (returns (MyTurn :type Boolean) (CurrentPlayerID :type String))
  (bind _currentturnplayerid (`/Game/_Main/GameMode/TCGGame/GameMode/GS_TCGGame_State.CurrentTurnPlayerID` (`self.GameState`)))
  (return (`KismetStringLibrary.EqualEqual_StrStr` _currentturnplayerid (`.playerID_29_60B8B3224464527C74F565A36E1F999C` (break `/Game/_Main/GameMode/TCGGame/Varaibles/ST_PlayerInfo` (`self.PlayerInfo`)))) _currentturnplayerid))

(fn `FN_RemoveAttribute`
  (params (Attribute :type "/Game/_Main/GameMode/TCGGame/Varaibles/E_PlayerAttribute Enum" :default "NewEnumerator0") (Amount :type Integer) (SkipRule :type Boolean :default true))
  (locals (TargetAttribute :type "/Game/_Main/GameMode/TCGGame/Varaibles/E_PlayerAttribute Enum" :default "NewEnumerator0") (RemoveAmount :type Integer) (SkipCheckingRule :type Boolean))
  (bind ((`playerAttribute_12_1398B0B949EE9B8A2B8F089301723C01` _playerattribute)) (break `/Game/_Main/GameMode/TCGGame/Varaibles/ST_PlayerInfo` (`self.PlayerInfo`)))
  (set `local.TargetAttribute` Attribute)
  (set `local.RemoveAmount` Amount)
  (set `local.SkipCheckingRule` SkipRule)
  (for (_array_element _array_index) _playerattribute
    (bind ((`name_12_77F2DFD944D268F5A3B1679009ADE39A` _name) (`current_11_F36D572A4C9F9C60EB314AB5DA8DC1DE` _current) (`Rules_16_2C41BDD843B56E4E4E4CFE94717A3310` _rules)) (break `/Game/_Main/GameMode/TCGGame/Varaibles/ST_PlayerAttributes` _array_element))
    (if (`|EnumEquality` _name (`local.TargetAttribute`))
      (if (`local.SkipCheckingRule`)
        (bind _returnvalue (- _current (`local.RemoveAmount`)))
        (setmembers `/Game/_Main/GameMode/TCGGame/Varaibles/ST_PlayerAttributes` :`StructRef` (`|GetArrayItem` _playerattribute _array_index) :`current` (`KismetMathLibrary.SelectInt` _returnvalue 0 (> _returnvalue 0)))
        (break)
        (else
          (`self.FN_HandleAttributeRule` _rules (`local.RemoveAmount`) _current (`local.TargetAttribute`))))))
  (`self.API_SyncClients_Client`))

(fn `FN_Spawn3DCardOnArea`
  (params (CardInfo :type "/Game/_Main/GameMode/TCGGame/Varaibles/ST_Card Structure") (isEnemy :type Boolean))
  (locals (IsEnemyFlag :type Boolean))
  (bind _widgetref (`self.WidgetRef`))
  (`/Engine/EditorBlueprintResources/StandardMacros.IsValid` _widgetref
    (:`Is Valid`
      (bind _output_get (set `local.IsEnemyFlag` isEnemy))
      (bind _outactors (`self.FN_GetNextSpawnPlace` _output_get))
      (bind _returnvalue (`Actor.GetTransform` _outactors))
      (bind _returnvalue_2 (`|SpawnActorFromClass` "/Game/_Main/GameMode/TCGGame/Actor/BP_Card.BP_Card_C" _returnvalue "AdjustIfPossibleButAlwaysSpawn" "MultiplyWithRoot" null CardInfo _widgetref (`local.IsEnemyFlag`) null))
      (`/Game/_Main/GameMode/TCGGame/Actor/BP_Card.API_PlayCardAnimation` _returnvalue_2 _returnvalue))))

(fn `FN_UseCardAttribute`
  (params (CardAttribute :type "/Game/_Main/GameMode/TCGGame/Varaibles/ST_CardRequired Structure"))
  (bind (_ispositiveaction _type _amount) (break `/Game/_Main/GameMode/TCGGame/Varaibles/ST_CardRequired` CardAttribute))
  (bind _returnvalue (* _amount -1))
  ; Only runs on the server
  (`/Engine/EditorBlueprintResources/ActorComponentMacros.Switch Has Authority`
    (:`Authority`
      (if _ispositiveaction
        (switch `/Game/_Main/GameMode/TCGGame/Varaibles/E_Type` _type
          (:`NewEnumerator0`
            (`self.API_ApplyDamage_Client` _amount))
          (:`NewEnumerator1`
            (`self.API_AddAtribute_Client` "NewEnumerator1" _amount))
          (:`NewEnumerator2`
            (`self.API_AddAtribute_Client` "NewEnumerator2" _amount)))
        (else
          (switch `/Game/_Main/GameMode/TCGGame/Varaibles/E_Type` _type
            (:`NewEnumerator0`
              (`self.API_AddAtribute_Client` "NewEnumerator0" _returnvalue))
            (:`NewEnumerator1`
              (`self.API_AddAtribute_Client` "NewEnumerator1" _returnvalue))
            (:`NewEnumerator2`
              (`self.API_AddAtribute_Client` "NewEnumerator2" _returnvalue))))))))

(fn `OnRep_GameMode`)

(fn `OnRep_GameState`)
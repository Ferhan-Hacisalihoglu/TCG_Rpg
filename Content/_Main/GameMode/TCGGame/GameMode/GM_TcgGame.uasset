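; Server game mode that referees a two-player trading card game match, against another player or a spawned AI.
; PostLogin registers players and starts multiplayer matches with a random first turn, while Tick refreshes timers and ends expired turns.
; Turn end rolls a die granting attribute points and bonus cards, then passes the turn through GameState, syncing clients and checking for a winner.
; Played cards spawn their own custom-rule actor to apply effects.
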(event `self.ReceiveTick`
  (params (DeltaSeconds :type "Float (single-precision)"))
  (bind _player01 (`self.Player01`))
  (bind _player02 (`self.Player02`))
  (bind _gamestatetcg (`self.GameStateTCG`))
  ; Update Turn leaft for all players
  (`/Engine/EditorBlueprintResources/StandardMacros.IsValid` _player01
    (:`Is Valid`
      (`/Game/_Main/GameMode/TCGGame/GameMode/BPC_TCG_Component.API_SetTimeLeftWidget_Client` _player01)
      (`/Engine/EditorBlueprintResources/StandardMacros.IsValid` _player02
        (:`Is Valid`
          (`/Game/_Main/GameMode/TCGGame/GameMode/BPC_TCG_Component.API_SetTimeLeftWidget_Client` _player02)
          (if (>= (`/Game/_Main/GameMode/TCGGame/GameMode/GS_TCGGame_State.CurrentTurnTime` _gamestatetcg) (`/Game/_Main/GameMode/TCGGame/GameMode/GS_TCGGame_State.TurnTimeLimit` _gamestatetcg))
            (`self.API_EndPlayerTurn`)))))))

(event `self.ReceiveBeginPlay`
  ; Spawn AI
  (bind _asgs_tcggame_state (cast `/Game/_Main/GameMode/TCGGame/GameMode/GS_TCGGame_State` (`GameplayStatics.GetGameState`)))
  (set `self.GameStateTCG` _asgs_tcggame_state)
  (if (`self.IsSinglePlayer`)
    (bind _returnvalue (`|SpawnActorFromClass` "/Game/_Main/GameMode/TCGGame/Actor/BP_AI.BP_AI_C" (`KismetMathLibrary.MakeTransform` (0.0 0.0 0.0)) "Undefined" "MultiplyWithRoot" null null))
    (`KismetSystemLibrary.Delay` 0.5)
    (bind _component (message `/Game/_Main/GameMode/TCGGame/GameMode/BPI_TCG_Controller.ReturnTCGController` (`Pawn.GetController` _returnvalue)))
    (set `self.Player02` _component)))

(event `API_StartMatch`
  ;[0.15 0.03689 0.09306 0.502] Tell game instance to start the match
  (`/Game/_Main/GameMode/TCGGame/GameMode/GS_TCGGame_State.API_StartMatch_Server` (`self.GameStateTCG`)))

(event `API_ISPlayerDead`
  ;[0.15 0.03689 0.09306 0.502] Set match winner
  (if (`self.IsPlayerDead` (`self.Player01`))
    (`/Game/_Main/GameMode/TCGGame/GameMode/GS_TCGGame_State.API_SetMatchWinner_Server` (`self.GameStateTCG`) (`.playerID_29_60B8B3224464527C74F565A36E1F999C` (break `/Game/_Main/GameMode/TCGGame/Varaibles/ST_PlayerInfo` (`/Game/_Main/GameMode/TCGGame/GameMode/BPC_TCG_Component.PlayerInfo` (`self.Player02`)))))
    (elif (`self.IsPlayerDead` (`self.Player02`))
      (`/Game/_Main/GameMode/TCGGame/GameMode/GS_TCGGame_State.API_SetMatchWinner_Server` (`self.GameStateTCG`) (`.playerID_29_60B8B3224464527C74F565A36E1F999C` (break `/Game/_Main/GameMode/TCGGame/Varaibles/ST_PlayerInfo` (`/Game/_Main/GameMode/TCGGame/GameMode/BPC_TCG_Component.PlayerInfo` (`self.Player01`))))))))

(event `API_SetPlayerTurn`
  (params (CurrentPlayerIndex :type String))
  ;[0.15 0.03689 0.09306 0.502] Comment
  (`/Game/_Main/GameMode/TCGGame/GameMode/GS_TCGGame_State.API_StartPlayerTurn_Server` (`self.GameStateTCG`) CurrentPlayerIndex)
  (`self.API_SyncClients`)
  (`/Game/_Main/GameMode/TCGGame/GameMode/BPC_TCG_Component.API_AddDrawNewCard_Client` (`self.FN_GetPlayerComponentID` CurrentPlayerIndex)))

(event `self.K2_PostLogin`
  (params (NewPlayer :type "PlayerController Object Reference"))
  ; Get players
  (bind _component (message `/Game/_Main/GameMode/TCGGame/GameMode/BPI_TCG_Controller.ReturnTCGController` NewPlayer))
  (`/Engine/EditorBlueprintResources/StandardMacros.IsValid` (`self.Player01`)
    (:`Is Valid`
      (set `self.Player02` _component))
    (:`Is Not Valid`
      (bind _output_get (set `self.Player01` _component))
      (`/Game/_Main/GameMode/TCGGame/GameMode/BPC_TCG_Component.API_HandleSession_Client` _output_get)))
  ; Start match with random player
  (`KismetSystemLibrary.Delay` 2.0)
  (if (and (not (`self.IsSinglePlayer`)) (`KismetSystemLibrary.IsValid` (`self.Player01`)) (`KismetSystemLibrary.IsValid` (`self.Player02`)))
    (`self.API_StartMatch`)
    (`self.API_SetPlayerTurn` (`KismetMathLibrary.SelectString` (`.playerID_29_60B8B3224464527C74F565A36E1F999C` (break `/Game/_Main/GameMode/TCGGame/Varaibles/ST_PlayerInfo` (`/Game/_Main/GameMode/TCGGame/GameMode/BPC_TCG_Component.PlayerInfo` (`self.Player01`)))) (`.playerID_29_60B8B3224464527C74F565A36E1F999C` (break `/Game/_Main/GameMode/TCGGame/Varaibles/ST_PlayerInfo` (`/Game/_Main/GameMode/TCGGame/GameMode/BPC_TCG_Component.PlayerInfo` (`self.Player02`)))) (`KismetMathLibrary.RandomBool`)))))

(event `API_EndPlayerTurn`
  ;[0.15 0.03689 0.09306 0.502] When player ends turn
  (set `self.LastPlayerID` (`/Game/_Main/GameMode/TCGGame/GameMode/GS_TCGGame_State.CurrentTurnPlayerID` (`self.GameStateTCG`)))
  (`self.API_SetPlayerTurn` "")
  (`KismetSystemLibrary.Delay` 0.5)
  (`self.API_Roll_Dice`)
  (`/Game/_Main/GameMode/TCGGame/GameMode/BPC_TCG_Component.API_RollDice` (`self.FN_GetPlayerComponentID` (`self.LastPlayerID`)))
  (`KismetSystemLibrary.Delay` 2.0)
  (if (`KismetStringLibrary.EqualEqual_StrStr` (`self.LastPlayerID`) (`.playerID_29_60B8B3224464527C74F565A36E1F999C` (break `/Game/_Main/GameMode/TCGGame/Varaibles/ST_PlayerInfo` (`/Game/_Main/GameMode/TCGGame/GameMode/BPC_TCG_Component.PlayerInfo` (`self.Player01`)))))
    (`self.API_SetPlayerTurn` (`.playerID_29_60B8B3224464527C74F565A36E1F999C` (break `/Game/_Main/GameMode/TCGGame/Varaibles/ST_PlayerInfo` (`/Game/_Main/GameMode/TCGGame/GameMode/BPC_TCG_Component.PlayerInfo` (`self.Player02`)))))
    (else
      (`self.API_SetPlayerTurn` (`.playerID_29_60B8B3224464527C74F565A36E1F999C` (break `/Game/_Main/GameMode/TCGGame/Varaibles/ST_PlayerInfo` (`/Game/_Main/GameMode/TCGGame/GameMode/BPC_TCG_Component.PlayerInfo` (`self.Player01`))))))))

(event `API_ApplyDamageEnemy`
  (params (SelfPlayer :type "/Game/_Main/GameMode/TCGGame/GameMode/BPC_TCG_Component Object Reference") (Amount :type Integer))
  ; Apply damage to enemy
  (bind _enemy (`self.FN_GetEnemy` SelfPlayer))
  (`/Game/_Main/GameMode/TCGGame/GameMode/BPC_TCG_Component.API_RemoveAttribute_Client` _enemy "NewEnumerator0" Amount false))

(event `API_Roll_Dice`
  ; Roll Dice
  (set `self.LastDiceRoll` (`KismetMathLibrary.RandomIntegerInRange` 1 6))
  (`KismetSystemLibrary.Delay` 1.0)
  (`self.FN_HandleDiceLogic`))

(event `API_HandleSession`)

(event `API_SyncClients`
  (bind _player02 (`self.Player02`))
  ; This will sync data on all clients
  (`self.API_ISPlayerDead`)
  (`/Game/_Main/GameMode/TCGGame/GameMode/BPC_TCG_Component.API_ReloadWidget_Client` (`self.Player01`))
  (`/Engine/EditorBlueprintResources/StandardMacros.IsValid` _player02
    (:`Is Valid`
      (`/Game/_Main/GameMode/TCGGame/GameMode/BPC_TCG_Component.API_ReloadWidget_Client` _player02)
      (`self.API_ISPlayerDead`))))

(event `API_FindEnemy`
  (params (SelfPlayer :type "/Game/_Main/GameMode/TCGGame/GameMode/BPC_TCG_Component Object Reference"))
  ;[0.15 0.06562 0.0375 0.5] Find Enemy on the server
  (bind _enemy (`self.FN_GetEnemy` SelfPlayer))
  (`/Game/_Main/GameMode/TCGGame/GameMode/BPC_TCG_Component.API_SetAndRefreshEnemy_Server` SelfPlayer _enemy))

(event `API_PlayerUserCard`
  (params (ST_Card :type "/Game/_Main/GameMode/TCGGame/Varaibles/ST_Card Structure") (Player :type "/Game/_Main/GameMode/TCGGame/GameMode/BPC_TCG_Component Object Reference"))
  ; When player use card
  (`/Game/_Main/GameMode/TCGGame/GameMode/BPC_TCG_Component.API_Spawn3DCard_Client` Player ST_Card true)
  (bind _enemy (`self.FN_GetEnemy` Player))
  (`/Game/_Main/GameMode/TCGGame/GameMode/BPC_TCG_Component.API_Spawn3DCard_Client` _enemy ST_Card false)
  (bind _returnvalue (`|SpawnActorFromClass` (`.CardCustomRules_35_F7AFF5044C77FF2D7AEABEADF0E91113` (break `/Game/_Main/GameMode/TCGGame/Varaibles/ST_Card` ST_Card)) (`KismetMathLibrary.MakeTransform` (0.0 0.0 0.0)) "Undefined" "MultiplyWithRoot" null null))
  (`/Game/_Main/GameMode/TCGGame/Actor/CardCustomRules/BP_BaseCardCustomRule.API_UseCustomRule_Server` _returnvalue Player _enemy))

(fn `FN_GetEnemy`
  (params (SelfPlayer :type "/Game/_Main/GameMode/TCGGame/GameMode/BPC_TCG_Component Object Reference"))
  (returns (Enemy :type "/Game/_Main/GameMode/TCGGame/GameMode/BPC_TCG_Component Object Reference"))
  (if (== (`self.Player01`) SelfPlayer)
    (return (`self.Player02`))
    (else
      (return (`self.Player01`)))))

(fn `FN_GetPlayerComponentID`
  (params (PlayerID :type String))
  (returns (`Player Return` :type "/Game/_Main/GameMode/TCGGame/GameMode/BPC_TCG_Component Object Reference"))
  (if (`KismetStringLibrary.EqualEqual_StrStr` PlayerID (`.playerID_29_60B8B3224464527C74F565A36E1F999C` (break `/Game/_Main/GameMode/TCGGame/Varaibles/ST_PlayerInfo` (`/Game/_Main/GameMode/TCGGame/GameMode/BPC_TCG_Component.PlayerInfo` (`self.Player01`)))))
    (return (`self.Player01`))
    (else
      (return (`self.Player02`)))))

(fn `FN_HandleDiceLogic`
  (bind _lastdiceroll (`self.LastDiceRoll`))
  (bind _player_return (`self.FN_GetPlayerComponentID` (`self.LastPlayerID`)))
  (`/Game/_Main/GameMode/TCGGame/GameMode/BPC_TCG_Component.API_AddAtribute_Client` _player_return "NewEnumerator1" _lastdiceroll)
  (if (> _lastdiceroll 4)
    (`/Game/_Main/GameMode/TCGGame/GameMode/BPC_TCG_Component.API_AddDrawNewCard_Client` _player_return)
    (`/Game/_Main/GameMode/TCGGame/GameMode/BPC_TCG_Component.API_AddDrawNewCard_Client` _player_return)
    (`/Game/_Main/GameMode/TCGGame/GameMode/BPC_TCG_Component.API_SendNotification` _player_return "NewEnumerator0" "You got two bonus card!")
    (elif (> _lastdiceroll 2)
      (`/Game/_Main/GameMode/TCGGame/GameMode/BPC_TCG_Component.API_AddDrawNewCard_Client` _player_return)
      (`/Game/_Main/GameMode/TCGGame/GameMode/BPC_TCG_Component.API_SendNotification` _player_return "NewEnumerator0" "You got a bonus card!"))))

(fn `UserConstructionScript`)